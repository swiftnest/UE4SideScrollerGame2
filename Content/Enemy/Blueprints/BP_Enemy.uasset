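; Side-scrolling walker enemy that stays idle until the player comes within range, then paces along the Y axis.
; A Start/Move/Dead state gates its events, and wall hit normals set the walking direction.
; Contact with UnityChanBlueprint damages the player, unless the hit normal points upward, in which case the enemy damages itself.
; Any damage while moving squashes it, plays a sound and destroys it after a short delay.
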(event `self.ReceiveTick`
  (params (DeltaSeconds :type "Float (single-precision)"))
  (switch `string` (`self.State`)
    (:`Start`
      ;[1 1 1] プレイヤーとの距離を判定してStateをMoveに変える
      (bind _returnvalue (`self.GetDistanceTo` (`GameplayStatics.GetPlayerPawn` 0)))
      (if (< _returnvalue 1000.0)
        (set `self.State` "Move")))
    (:`Move`
      ;[1 1 1] 左右移動
      (`self.AddMovementInput` (0.0 0.2 0.0) (`self.Direction`)))))

(event `self.ReceiveHit`
  (params (MyComp :type "PrimitiveComponent Object Reference") (Other :type "Actor Object Reference") (OtherComp :type "PrimitiveComponent Object Reference") (bSelfMoved :type Boolean) (HitLocation :type "Object.Vector Structure") (HitNormal :type "Object.Vector Structure") (NormalImpulse :type "Object.Vector Structure") (Hit :type "EngineTypes.HitResult Structure (by ref)"))
  (bind _y (.y HitNormal))
  (switch `string` (`self.State`)
    (:`Move`
      ;[1 1 1] 攻撃＆ダメージ処理
      (bind _asunitychanblueprint_c (cast `/Game/UnityChan/Blueprints/UnityChanBlueprint` Other)
        (:`then`
          (if (> (.z HitNormal) 0.6)
            (`GameplayStatics.ApplyDamage` self 1.0)
            (else
              (`GameplayStatics.ApplyDamage` _asunitychanblueprint_c 1.0))))
        (:`CastFailed`
          ;[1 1 1] 左右反転
          (if (< _y -0.5)
            (set `self.Direction` -1.0)
            (elif (> _y 0.5)
              (set `self.Direction` 1.0))))))))

(event `self.ReceiveAnyDamage`
  (params (Damage :type "Float (single-precision)") (DamageType :type "DamageType Object Reference") (InstigatedBy :type "Controller Object Reference") (DamageCauser :type "Actor Object Reference"))
  (switch `string` (`self.State`)
    (:`Move`
      ;[1 1 1] 死亡処理
      (set `self.State` "Dead")
      (`SceneComponent.AddLocalOffset` (`self.StaticMesh1`) (0.0 0.0 -50.0) false)
      (`self.SetActorScale3D` (`KismetMathLibrary.MakeVector` 1.0 1.0 0.5))
      (`GameplayStatics.PlaySoundAtLocation` "/Game/Audio/damage.Damage" (`self.K2_GetActorLocation`))
      (`KismetSystemLibrary.Delay` 0.5)
      (`self.K2_DestroyActor`))))

(fn `UserConstructionScript`)