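; BP_MoveFloor is a moving floor gimmick that slides along the world Y axis relative to where it starts.
; BeginPlay caches the start location and seeks the timeline to StartTime, so the motion can begin at an offset.
; Tick calls Play on the timeline every frame, and each update sets the location from the track value scaled toward negative Y, without sweep.
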(event `self.ReceiveBeginPlay`
  (set `self.StartLocation` (`self.K2_GetActorLocation`))
  (`TimelineComponent.SetNewTime` (`self.Timeline_0`) (`self.StartTime`)))

(event `self.ReceiveTick`
  (params (DeltaSeconds :type "Float (single-precision)"))
  (bind (_direction _newtrack_0) (`Timeline|Timeline_0` :`NewTime` DeltaSeconds)
    (:`Update`
      (`self.K2_SetActorLocation` (+ (`KismetMathLibrary.MakeVector` 0.0 (* _newtrack_0 -500.0)) (`self.StartLocation`))))))

(fn `UserConstructionScript`)